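; Player pawn that is constantly pushed along the negative of its yaw-only control forward vector at half input scale every Tick.
; Forward, left and right input axes add movement relative to the control yaw.
; Pressing A or D plays the Left or Right timeline, which rolls the Untitled component about the world X axis to tilt it, and releasing reverses that timeline.
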(event EventTick
  (params (DeltaSeconds :type Float%20%28single-precision%29))
  (Pawn|Input|AddMovementInput (Math|Vector|GetForwardVector (Math|Rotator|MakeRotator 0.0 0.0 (.Yaw (Math|Rotator|BreakRotator (Pawn|GetControlRotation :!class /Script/Engine.Pawn))))) -0.5 false))

(event Input|AxisEvents|InputAxisforward
  (params (AxisValue :type Float%20%28single-precision%29))
  (Pawn|Input|AddMovementInput (Math|Vector|GetForwardVector (Math|Rotator|MakeRotator 0.0 0.0 (.Yaw (Math|Rotator|BreakRotator (Pawn|GetControlRotation :!class /Script/Engine.Pawn))))) AxisValue false))

(event Input|AxisEvents|InputAxisleft
  (params (AxisValue :type Float%20%28single-precision%29))
  (Pawn|Input|AddMovementInput (Math|Vector|GetRightVector (Math|Rotator|MakeRotator 0.0 0.0 (.Yaw (Math|Rotator|BreakRotator (Pawn|GetControlRotation :!class /Script/Engine.Pawn))))) AxisValue false))

(event Input|AxisEvents|InputAxisright
  (params (AxisValue :type Float%20%28single-precision%29))
  (Pawn|Input|AddMovementInput (Math|Vector|GetRightVector (Math|Rotator|MakeRotator 0.0 0.0 (.Yaw (Math|Rotator|BreakRotator (Pawn|GetControlRotation :!class /Script/Engine.Pawn))))) AxisValue false))

(event Input|KeyboardEvents|A
  (params (Key :type Key%20Structure :default "None"))
  (:Pressed
    (bind _left_vec (Timeline|left PlayFromStart)
      (:Update
        _)
      (:Finished
        _))
    (Transformation|SetWorldRotation (Variables|Default|Getuntitled) (Math|Vector|RotatorfromAxisandAngle "5.000000, 0, 0" _left_vec) false false))
  (:Released
    (Timeline|left Reverse)))

(event Input|KeyboardEvents|D
  (params (Key :type Key%20Structure :default "None"))
  (:Pressed
    (bind _left_vec (Timeline|right Play)
      (:Update
        _)
      (:Finished
        _))
    (Transformation|SetWorldRotation (Variables|Default|Getuntitled) (Math|Vector|RotatorfromAxisandAngle "5.000000, 0, 0" _left_vec) false false))
  (:Released
    (Timeline|right Reverse)))

(fn ConstructionScript)